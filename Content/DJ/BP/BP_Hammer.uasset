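; BP_Hammer is a hammer weapon actor that deals damage to whatever its mesh hits.
; On a HammerMesh hit, it prints a debug string and applies fixed damage, naming the player character as damage causer.
; It then briefly simulates physics on the mesh at a partial blend weight, switching it off after a short delay to give a physical impact reaction.
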(event `self.ReceiveBeginPlay`)

(event `self.HammerMesh.OnComponentHit`
  (params (HitComponent :type "PrimitiveComponent Object Reference") (OtherActor :type "Actor Object Reference") (OtherComp :type "PrimitiveComponent Object Reference") (NormalImpulse :type "Vector Structure") (Hit :type "HitResult Structure (by ref)"))
  (`KismetSystemLibrary.PrintString` "Hello")
  ; 무기 물리엔진
  (`GameplayStatics.ApplyDamage` OtherActor 10.0 null (`GameplayStatics.GetPlayerCharacter` 0))
  (`PrimitiveComponent.SetSimulatePhysics` (`self.HammerMesh`) true)
  (`SkeletalMeshComponent.SetPhysicsBlendWeight` (`self.HammerMesh`) 0.3)
  (`KismetSystemLibrary.Delay` 0.15)
  (`SkeletalMeshComponent.SetPhysicsBlendWeight` (`self.HammerMesh`) 0.0)
  (`PrimitiveComponent.SetSimulatePhysics` (`self.HammerMesh`) false))

(fn `UserConstructionScript`)