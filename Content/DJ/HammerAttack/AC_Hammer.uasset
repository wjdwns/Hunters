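; Actor component that gives its owning Character a hammer by spawning one and attaching it to the character's mesh.
; On BeginPlay it casts the owner to Character, stores the reference and calls NewFunction, which spawns the configured hammer class and keeps a reference to it.
; The hammer snaps to a named socket on the mesh; the component contains no attack logic.
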(event `self.ReceiveBeginPlay`
  (bind _ascharacter (cast `Character` (`self.GetOwner`)))
  (set `self.CharacterRef` _ascharacter)
  (`self.NewFunction`))

(fn `NewFunction`
  (bind _returnvalue (`|SpawnActorFromClass` (`self.HammerClass`) (`KismetMathLibrary.MakeTransform` (0.0 0.0 0.0)) "Undefined" "MultiplyWithRoot" null null))
  (bind _output_get (set `self.HammerRef` _returnvalue))
  (`Actor.K2_AttachToComponent` _output_get (`Character.Mesh` (`self.CharacterRef`)) (`self.HammerSocketName`) "SnapToTarget" "SnapToTarget" "SnapToTarget" true))