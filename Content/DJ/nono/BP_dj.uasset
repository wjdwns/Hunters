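; BP_dj is a player pawn prototype with movement, yaw-only look and a charged hammer attack stubbed out with debug prints.
; BeginPlay sets game-only input and adds the IMC_Hammer Enhanced Input context; movement follows control yaw.
; Holding IA_Hammer_New accumulates ChargeTime, and release chooses a heavy or light attack message.
; The release check compares ChargeTime to itself, so the light branch always runs.
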(event `Key|Q`
  (params (Key :type "Key Structure")))

(event `Key|LeftMouseButton`
  (params (Key :type "Key Structure")))

(event `self.ReceiveTick`
  (params (DeltaSeconds :type "Float (single-precision)")))

(event `self.ReceiveBeginPlay`
  (bind _returnvalue (`GameplayStatics.GetPlayerController` 0))
  ;[0.1449 0.05075 0.15 0.5] wasd
  (`WidgetBlueprintLibrary.SetInputMode_GameOnly` _returnvalue)
  (`EnhancedInputSubsystemInterface.AddMappingContext` (pcsubsystem `EnhancedInputLocalPlayerSubsystem` _returnvalue) "/Game/DJ/nono/IMC_Hammer.IMC_Hammer" 999 (struct))
  (`KismetSystemLibrary.PrintString` "addmappingcontext"))

(event `EnhancedInput|/Game/DJ/nono/IA_Hammer_New`
  (params (ActionValue :type Boolean) (ElapsedSeconds :type "Float (double-precision)") (TriggeredSeconds :type "Float (double-precision)") (InputAction :type "InputAction Object Reference" :default "/Game/DJ/nono/IA_Hammer_New.IA_Hammer_New"))
  (bind _chargetime (`self.ChargeTime`))
  ; 차징
  (:`Triggered`
    (set `self.ChargeTime` (+ (`GameplayStatics.GetWorldDeltaSeconds`) (`self.ChargeTime`)))
    (`KismetSystemLibrary.PrintString` "Hello"))
  (:`Started`
    (set `self.ChargeTime` 0.0)
    (`KismetSystemLibrary.PrintString` "차지시작"))
  (:`Completed`
    (if (> _chargetime _chargetime)
      (`KismetSystemLibrary.PrintString` "3단계 강공격!!")
      (else
        (`KismetSystemLibrary.PrintString` "1단계 약공격!!")))
    (set `self.ChargeTime` 0.0)))

(event `EnhancedInput|/Game/DJ/nono/dj_move`
  (params (ActionValue :type "Vector2D Structure") (ElapsedSeconds :type "Float (double-precision)") (TriggeredSeconds :type "Float (double-precision)") (InputAction :type "InputAction Object Reference" :default "/Game/DJ/nono/dj_move.dj_move"))
  (bind _returnvalue (`KismetMathLibrary.MakeRotator` 0.0 0.0 (.yaw (`self.GetControlRotation`))))
  ;[0.1449 0.05075 0.15 0.5] wasd
  (:`Triggered`
    (`self.AddMovementInput` (`KismetMathLibrary.GetRightVector` _returnvalue) ActionValue_X)
    (`self.AddMovementInput` (`KismetMathLibrary.GetForwardVector` _returnvalue) ActionValue_Y)))

(event `EnhancedInput|/Game/Input/Actions/IA_Look`
  (params (ActionValue :type "Vector2D Structure") (ElapsedSeconds :type "Float (double-precision)") (TriggeredSeconds :type "Float (double-precision)") (InputAction :type "InputAction Object Reference" :default "/Game/Input/Actions/IA_Look.IA_Look"))
  ;[0.1449 0.05075 0.15 0.5] wasd
  (:`Triggered`
    (`self.AddControllerYawInput` ActionValue_X)))

(fn `UserConstructionScript`)