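; BP_Arrow is an arrow projectile actor that stays without projectile movement until its Fire event is called with a direction and strength.
; Fire adds a ProjectileMovement component at runtime, using strength to blend launch speed from min to max and gravity scale from max to min, so stronger shots fly faster and flatter.
; It also spawns a trail effect attached at the TrailEffectLocation component.
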(event `Fire`
  (params (Direction :type "Vector Structure") (Strangth :type "Float (double-precision)"))
  (bind _returnvalue (`AddComponent|NODE_AddProjectileMovementComponent-0`))
  (set `MovementComponent.Velocity` (* Direction (`KismetMathLibrary.Lerp` (`self.MinSpeed`) (`self.MaxSpeed`) Strangth)) _returnvalue)
  (set `ProjectileMovementComponent.ProjectileGravityScale` (`KismetMathLibrary.Lerp` (`self.MaxGravity`) (`self.MinGravity`) Strangth) _returnvalue)
  (`NiagaraFunctionLibrary.SpawnSystemAttached` (`self.TrailEffect`) (`self.TrailEffectLocation`) "None" (0.0 0.0 0.0) (struct) "KeepRelativeOffset"))

(fn `UserConstructionScript`)