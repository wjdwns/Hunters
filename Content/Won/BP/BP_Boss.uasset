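; BP_Boss is a player-controlled boss character with camera-relative movement and a tongue attack, using Enhanced Input.
; Tick also adds movement from the raw axis values and turns the actor toward its velocity.
; After two seconds without look input, control rotation interpolates to bring the camera back behind.
; The fire input spawns and attaches a BP_Tougue actor, destroying it when TongueTimeline finishes.
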(event `EnhancedInput|/Game/Won/Input/Move_Forward`
  (params (ActionValue :type "Float (double-precision)") (ElapsedSeconds :type "Float (double-precision)") (TriggeredSeconds :type "Float (double-precision)") (InputAction :type "InputAction Object Reference" :default "/Game/Won/Input/Move_Forward.Move_Forward"))
  (:`Triggered`
    (`self.AddMovementInput` (`KismetMathLibrary.GetForwardVector` (`KismetMathLibrary.MakeRotator` 0.0 0.0 (.yaw (`self.GetControlRotation`)))) ActionValue)))

(event `Tongue Fire`)

(event `EnhancedInput|/Game/Won/Input/Move_Sides`
  (params (ActionValue :type "Float (double-precision)") (ElapsedSeconds :type "Float (double-precision)") (TriggeredSeconds :type "Float (double-precision)") (InputAction :type "InputAction Object Reference" :default "/Game/Won/Input/Move_Sides.Move_Sides"))
  (:`Triggered`
    (`self.AddMovementInput` (`KismetMathLibrary.GetRightVector` (`KismetMathLibrary.MakeRotator` 0.0 0.0 (.yaw (`self.GetControlRotation`)))) ActionValue)))

(event `self.ReceiveBeginPlay`
  ; 컨트롤
  (`|ExecutionSequence`
    (:`then_0`
      (`EnhancedInputSubsystemInterface.AddMappingContext` (pcsubsystem `EnhancedInputLocalPlayerSubsystem` (`GameplayStatics.GetPlayerController` 0)) "/Game/Won/Input/Move_Context.Move_Context" 0 (struct)))
    (:`then_1`
      (`SceneComponent.K2_SetRelativeLocation` (`self.Tongue_cube`) (50.0 0.0 0.0) false false))))

(event `EnhancedInput|/Game/Won/Input/Tougue_Fire`
  (params (ActionValue :type "Float (double-precision)") (ElapsedSeconds :type "Float (double-precision)") (TriggeredSeconds :type "Float (double-precision)") (InputAction :type "InputAction Object Reference" :default "/Game/Won/Input/Tougue_Fire.Tougue_Fire"))
  ; 혓바닥 발사
  (:`Started`
    (bind _returnvalue (`|SpawnActorFromClass` "/Game/Won/BP/BP_Tougue.BP_Tougue_C" (`SceneComponent.K2_GetComponentToWorld` (`self.Tougue`)) "Undefined" "MultiplyWithRoot" null null))
    (`self.K2_AttachToComponent` _returnvalue null "None" "SnapToTarget" "SnapToTarget" "SnapToTarget" true)
    (`Timeline|TongueTimeline` :!via `PlayFromStart`
      (:`Finished`
        (`self.K2_DestroyActor` _returnvalue)))))

(event `self.ReceiveTick`
  (params (DeltaSeconds :type "Float (single-precision)"))
  (bind _returnvalue (`self.GetVelocity`))
  ; 움직임 설정
  (`|ExecutionSequence`
    (:`then_0`
      (`self.AddMovementInput` (`KismetMathLibrary.Normal` (`KismetMathLibrary.MakeVector` (`|GetInputActionValue`) (`|GetInputActionValue`))) (`self.Speed`))
      (if (> (`KismetMathLibrary.VSize` _returnvalue) 0.0)
        (`self.K2_SetActorRotation` (`KismetMathLibrary.MakeRotator` 0.0 0.0 (.yaw (`KismetMathLibrary.Conv_VectorToRotator` _returnvalue))))))
    (:`then_1`
      ; 카메라 뒤로 자동이동
      (if (> (- (`KismetSystemLibrary.GetGameTimeInSeconds`) (`self.LastInputTime`)) 2.0)
        (`Controller.SetControlRotation` (`GameplayStatics.GetPlayerController` 0) (`KismetMathLibrary.RInterpTo` (struct) (struct) DeltaSeconds))))))

(event `EnhancedInput|/Game/Won/Input/IA_Look`
  (params (ActionValue :type "Vector2D Structure") (ElapsedSeconds :type "Float (double-precision)") (TriggeredSeconds :type "Float (double-precision)") (InputAction :type "InputAction Object Reference" :default "/Game/Won/Input/IA_Look.IA_Look"))
  (:`Triggered`
    (set `self.LastInputTime` (`KismetSystemLibrary.GetGameTimeInSeconds`))
    (`self.AddControllerYawInput` ActionValue_X)
    (`self.AddControllerPitchInput` ActionValue_Y)))

(fn `UserConstructionScript`)