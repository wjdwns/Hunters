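; Player-controlled frog boss character with camera-relative or input-driven movement, facing its velocity, and idle camera realignment after look input stops.
; Tongue attack attaches a temporary BP_Tougue actor for a timeline; its input event is empty.
; Key 1 runs a timeline tackle that damages overlapped BP_Dong and BP_Player, knocking the player back.
; Key 2 launches a jump via the JumpAttack component, landing with particles and camera shake; its radial damage is unwired.
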(event `EnhancedInput|/Game/Won/Input/Tougue_Fire`
  (params (ActionValue :type "Float (double-precision)") (ElapsedSeconds :type "Float (double-precision)") (TriggeredSeconds :type "Float (double-precision)") (InputAction :type "InputAction Object Reference" :default "/Game/Won/Input/Tougue_Fire.Tougue_Fire")))

(event `Attack_Tongue`
  ; 혓바닥 발사
  (bind _returnvalue (`|SpawnActorFromClass` "/Game/Won/BP/BP_Tougue.BP_Tougue_C" (`SceneComponent.K2_GetComponentToWorld` (`self.Tougue`)) "Undefined" "MultiplyWithRoot" null null))
  (`self.K2_AttachToComponent` _returnvalue null "None" "SnapToTarget" "SnapToTarget" "SnapToTarget" true)
  (`Timeline|TongueTimeline` :!via `PlayFromStart`
    (:`Finished`
      (`self.K2_DestroyActor` _returnvalue))))

(event `self.Tackle_Zone.OnComponentBeginOverlap`
  (params (OverlappedComponent :type "PrimitiveComponent Object Reference") (OtherActor :type "Actor Object Reference") (OtherComp :type "PrimitiveComponent Object Reference") (OtherBodyIndex :type Integer) (bFromSweep :type Boolean) (SweepResult :type "HitResult Structure (by ref)"))
  ; 몸통박치기
  (`|ExecutionSequence`
    (:`then_0`
      (if (`self.Is_Tackle?`)
        (bind _asbp_dong (cast `/Game/DJ/BP/BP_Dong` OtherActor))
        (`GameplayStatics.ApplyDamage` _asbp_dong 10.0)))
    (:`then_1`
      (if (`self.Is_Tackle?`)
        (bind _asbp_player (cast `/Game/Jun/Player/BP_Player` OtherActor))
        (`GameplayStatics.ApplyDamage` null 10.0)
        (`KismetSystemLibrary.PrintString` "맞았다")
        (`Character.LaunchCharacter` _asbp_player (* (`self.GetActorForwardVector`) (`self.Tackle_Knock-Back`)) false false)))))

(event `Key|One`
  (params (Key :type "Key Structure"))
  ; 몸통박치기
  (:`Pressed`
    (set `self.Is_Tackle?` true)
    (bind (_direction _tackle_speed) (`Timeline|Tackle_Timeline` :!via `PlayFromStart`)
      (:`Update`
        (`self.K2_AddActorWorldOffset` (* _tackle_speed (* (`self.GetActorForwardVector`) (`self.Float(Tackle)`)))))
      (:`Finished`
        (set `self.Is_Tackle?` false)))))

(event `self.ReceiveBeginPlay`
  ; 컨트롤
  (`|ExecutionSequence`
    (:`then_0`
      (`EnhancedInputSubsystemInterface.AddMappingContext` (pcsubsystem `EnhancedInputLocalPlayerSubsystem` (`GameplayStatics.GetPlayerController` 0)) "/Game/Won/Input/Move_Context.Move_Context" 0 (struct)))
    (:`then_1`
      (`SceneComponent.K2_SetRelativeLocation` (`self.Boss_Body`) (50.0 0.0 0.0) false false))))

(event `self.Boss_Body.OnComponentHit`
  (params (HitComponent :type "PrimitiveComponent Object Reference") (OtherActor :type "Actor Object Reference") (OtherComp :type "PrimitiveComponent Object Reference") (NormalImpulse :type "Vector Structure") (Hit :type "HitResult Structure (by ref)"))
  (bind (_returnvalue_x _returnvalue_y) (`KismetMathLibrary.BreakVector` (`self.K2_GetActorLocation`)))
  ; 점프공격
  (set `self.Is_Jumping?` false)
  (`ActorComponent.Deactivate` (`self.JumpAttack`))
  (`MovementComponent.StopMovementImmediately` (`self.JumpAttack`))
  (`GameplayStatics.SpawnEmitterAtLocation` "/Engine/Tutorial/SubEditors/TutorialAssets/TutorialParticleSystem.TutorialParticleSystem" (`KismetMathLibrary.MakeVector` (.x (`KismetMathLibrary.MakeVector` _returnvalue_x _returnvalue_y -80.0)) (.y (`KismetMathLibrary.MakeVector` _returnvalue_x _returnvalue_y -80.0)) (.z (`KismetMathLibrary.MakeVector` _returnvalue_x _returnvalue_y -80.0))))
  (`GameplayStatics.PlayWorldCameraShake` "/Game/Won/BP/BP_CS_BossLand.BP_CS_BossLand_C" (0.0 0.0 0.0) 1500.0 7000.0))

(event `Key|Two`
  (params (Key :type "Key Structure"))
  ; 점프공격
  (:`Pressed`
    (set `self.Is_Jumping?` true)
    (`ProjectileMovementComponent.SetVelocityInLocalSpace` (`self.JumpAttack`) (800.0 0.0 1000.0))
    (`ActorComponent.Activate` (`self.JumpAttack`) false)))

(event `self.ReceiveTick`
  (params (DeltaSeconds :type "Float (single-precision)"))
  (bind _returnvalue (`self.GetVelocity`))
  ; 움직임 설정
  (`|ExecutionSequence`
    (:`then_0`
      (if (not (`self.Is_Jumping?`))
        (`self.AddMovementInput` (`KismetMathLibrary.Normal` (`KismetMathLibrary.MakeVector` (`|GetInputActionValue`) (`|GetInputActionValue`))) (`self.Speed`))
        ; 보스 360도 세팅
        (if (> (`KismetMathLibrary.VSize` _returnvalue) 0.0)
          (`self.K2_SetActorRotation` (`KismetMathLibrary.MakeRotator` 0.0 0.0 (.yaw (`KismetMathLibrary.Conv_VectorToRotator` _returnvalue)))))))
    (:`then_1`
      ; 카메라 뒤로 자동이동
      (if (> (- (`KismetSystemLibrary.GetGameTimeInSeconds`) (`self.LastInputTime`)) 20.0)
        (`Controller.SetControlRotation` (`GameplayStatics.GetPlayerController` 0) (`KismetMathLibrary.RInterpTo` (struct) (struct) DeltaSeconds))))))

(event `EnhancedInput|/Game/Won/Input/IA_Look`
  (params (ActionValue :type "Vector2D Structure") (ElapsedSeconds :type "Float (double-precision)") (TriggeredSeconds :type "Float (double-precision)") (InputAction :type "InputAction Object Reference" :default "/Game/Won/Input/IA_Look.IA_Look"))
  ; 카메라 시점변경
  (:`Triggered`
    (set `self.LastInputTime` (`KismetSystemLibrary.GetGameTimeInSeconds`))
    (`self.AddControllerYawInput` ActionValue_X)
    (`self.AddControllerPitchInput` ActionValue_Y)))

(fn `UserConstructionScript`)