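; BP_PatrolRoute is a patrol path actor that holds a spline and a current point index for AI to follow.
; GetSplinePontAsWorldPosition returns that point's world location, and IncrementPatrolRoute steps the index by a direction value.
; The ping-pong reversal is incomplete: the end-of-spline check is unconnected and the branch is fixed true, so direction becomes -1 after every step and the start-point reversal never runs.
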(event `IncrementPatrolRoute`
  (bind _output_get (set `self.PatrolIndex` (+ (`self.PatrolIndex`) (`self.Direrction`))))
  (if true
    (set `self.Direrction` -1)
    (elif (== (`self.PatrolIndex`) 0)
      (set `self.Direrction` 1))))

(fn `GetSplinePontAsWorldPosition`
  (returns (Location :type "Vector Structure"))
  (return (`SplineComponent.GetLocationAtSplinePoint` (`self.PatrolRoute`) (`self.PatrolIndex`) "World")))

(fn `UserConstructionScript`)