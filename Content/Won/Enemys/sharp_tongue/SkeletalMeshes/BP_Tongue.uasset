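; BP_Tongue is a short-lived tongue attack actor, apparently for the sharp tongue enemy, that damages what it overlaps.
; It expires after 1.5 seconds, or earlier if Tick finds its BP_Enemy_Base instigator dead, disabling collision before destroying itself.
; On overlapping a non-instigator, CollisionBox disables its own collision to hit only once, then sends a Strength-based damage message to the sweep result's hit actor.
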(event `self.ReceiveBeginPlay`
  (`self.SetLifeSpan` 1.5))

(event `self.ReceiveTick`
  (params (DeltaSeconds :type "Float (single-precision)"))
  (bind _asbp_enemy_base (cast `/Game/Won/Enemys/BP_Enemy_Base` (`self.GetInstigator`)))
  (if (`/Game/Won/Enemys/BP_Enemy_Base.IsDead` _asbp_enemy_base)
    (`PrimitiveComponent.SetCollisionEnabled` (`self.SkeletalMesh`) "NoCollision")
    (`PrimitiveComponent.SetCollisionEnabled` (`self.Box1`) "NoCollision")
    (`PrimitiveComponent.SetCollisionEnabled` (`self.CollisionBox`) "NoCollision")
    (`self.K2_DestroyActor`)))

(event `self.CollisionBox.OnComponentBeginOverlap`
  (params (OverlappedComponent :type "PrimitiveComponent Object Reference") (OtherActor :type "Actor Object Reference") (OtherComp :type "PrimitiveComponent Object Reference") (OtherBodyIndex :type Integer) (bFromSweep :type Boolean) (SweepResult :type "HitResult Structure (by ref)"))
  (if (!= OtherActor (`self.GetInstigator`))
    (`PrimitiveComponent.SetCollisionEnabled` (`self.CollisionBox`) "NoCollision")
    (message `/Game/Jun/DamageSystem/BPI_Damagable.TakeDamage` (`.HitActor` (`GameplayStatics.BreakHitResult` SweepResult)) (make `/Game/Jun/DamageSystem/S_DamageInfo` (`self.Strength`) "NewEnumerator2" "NewEnumerator1"))))

(fn `UserConstructionScript`)